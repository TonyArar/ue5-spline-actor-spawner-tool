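; Editor tool actor that fills a spline with a set number of copies of a chosen actor.
; Uniform scale comes from spline length divided by the actor's bounding-box X times the count, and each copy advances by that scaled length.
; The construction script previews copies as child actor components in local space.
; PlaceActors, meant to be run manually in editor, spawns real world-space actors, optionally rotated along the spline tangent.
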(fn ConstructionScript
  (Utilities|FlowControl|Sequence
    (:then_0
      ;[1 1 1 0.2] Operation #1: Preview Spawn
      (CallFunction|PreviewActorsPlacement))
    (:then_1)))

(fn PlaceActors
  (bind _actor_to_spawn (Variables|Default|GetActor%20To%20Spawn))
  (bind _actor_bounding_box_dimensions (CallFunction|CalculateActorBoundingBoxDimensionVector _actor_to_spawn))
  (bind _scale_per_actor (CallFunction|CalculateScalePerActor (Spline|GetSplineLength (Variables|Default|GetSpline)) _actor_bounding_box_dimensions (Variables|Default|GetNumber%20Of%20Actrors%20To%20Spawn)))
  (LocalVariables|SetActor%20Scale (Math|Vector|MakeVector _scale_per_actor _scale_per_actor _scale_per_actor)) ; calculated scale per actor
  (LocalVariables|SetAccumulated%20Distance 0.0) ; Initialize Accumulated Distance to 0
  (for _index (range 1 (Variables|Default|GetNumber%20Of%20Actrors%20To%20Spawn))
    (|SpawnActor (LocalVariables|GetActor%20Scale) (LocalVariables|GetAccumulated%20Distance) (Variables|Default|GetRotate%20Along%20Spline)) ; spawn actor in world space (game)
    (LocalVariables|SetAccumulated%20Distance (CallFunction|CalculateNewAccumulatedDistance (LocalVariables|GetAccumulated%20Distance) (.X (Math|Vector|BreakVector (* (Math|Vector|MakeVector _scale_per_actor _scale_per_actor _scale_per_actor) _actor_bounding_box_dimensions))))) ; update Accumulated Distance
  ))

(fn PreviewActorsPlacement
  (bind _actor_to_spawn (Variables|Default|GetActor%20To%20Spawn))
  (bind _actor_bounding_box_dimensions (CallFunction|CalculateActorBoundingBoxDimensionVector _actor_to_spawn))
  (bind _scale_per_actor (CallFunction|CalculateScalePerActor (Spline|GetSplineLength (Variables|Default|GetSpline)) _actor_bounding_box_dimensions (Variables|Default|GetNumber%20Of%20Actrors%20To%20Spawn)))
  (LocalVariables|SetActor%20Scale (Math|Vector|MakeVector _scale_per_actor _scale_per_actor _scale_per_actor)) ; calculated scale per actor
  (LocalVariables|SetAccumulated%20Distance 0.0) ; Initialize Accumulated Distance to 0
  (for _index (range 1 (Variables|Default|GetNumber%20Of%20Actrors%20To%20Spawn))
    (|Preview-SpawnActor (LocalVariables|GetActor%20Scale) (LocalVariables|GetAccumulated%20Distance) (Variables|Default|GetRotate%20Along%20Spline)) ; spawn actor in local space, can serve as preview
    (LocalVariables|SetAccumulated%20Distance (CallFunction|CalculateNewAccumulatedDistance (LocalVariables|GetAccumulated%20Distance) (.X (Math|Vector|BreakVector (* (Math|Vector|MakeVector _scale_per_actor _scale_per_actor _scale_per_actor) _actor_bounding_box_dimensions))))) ; update Accumulated Distance
  ))

(fn CalculateActorSpawnTransformatSplineDistance
  (params (Actor%20Scale :type Vector) (Accumulated%20Distance :type Float%20%28single-precision%29) (Rotate%20Along%20Spline%20Tangent :type Boolean) (Local%20Space%20Transform :type Boolean))
  (if Local%20Space%20Transform
    (LocalVariables|SetCoordinate%20Space "Local"))
  (bind _transform (Math|Transform|MakeTransform (LocalVariables|GetCoordinate%20Space) Accumulated%20Distance Rotate%20Along%20Spline%20Tangent Actor%20Scale)
    (:exit
      (return _transform))))

(fn CalculateNewAccumulatedDistance
  (params (Current%20Accumulated%20Distance :type Float%20%28double-precision%29) (Actor%20X%20Dimension :type Float%20%28double-precision%29))
  (return (+ Current%20Accumulated%20Distance Actor%20X%20Dimension)))

(fn CalculateActorBoundingBoxDimensionVector
  (params (Actor :type Actor%20Object%20Reference))
  (bind _boxextent (Collision|GetActorBounds Actor false false))
  (return (Math|Vector|VectorGetAbs (+ _boxextent _boxextent))))

(fn CalculateScalePerActor
  (params (Spline%20Length :type Float%20%28double-precision%29) (Actor%20Dimensions :type Vector) (Number%20Of%20Actors%20To%20Spawn :type Integer))
  (return (/ Spline%20Length (* (.X (Math|Vector|BreakVector Actor%20Dimensions)) (Math|Conversions|ToFloat(Integer) Number%20Of%20Actors%20To%20Spawn)))))