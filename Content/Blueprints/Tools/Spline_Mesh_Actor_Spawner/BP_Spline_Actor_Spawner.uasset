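; Editor tool that places copies of a chosen actor class at even intervals along a spline, optionally rotated to its tangent.
; The construction script previews the layout with child actor components in local space.
; PlaceActors, meant to be triggered manually in the editor, spawns real actors in world space.
; Both derive the count from spline length divided by a step of minimum bounding-box distance plus Spacing, assuming centered pivots.
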(fn ConstructionScript
  (Utilities|FlowControl|Sequence
    (:then_0
      ;[1 1 1 0.2] Operation #1: Preview Spawn
      (CallFunction|PreviewActorsPlacement))
    (:then_1)))

(fn PlaceActors
  (bind _scale (Variables|Default|GetScale))
  (LocalVariables|SetAccumulated%20Distance 0.0) ; Initialize Accumulated Distance to 0
  (bind (_number_of_actors_to_place _offset_distance_between_actors) (|CalculateOffsetDistanceAndNumberOfActors _scale (Variables|Default|GetActor%20To%20Spawn)))
  (for _index (range 1 _number_of_actors_to_place)
    (|SpawnActor _scale (LocalVariables|GetAccumulated%20Distance) (Variables|Default|GetRotate%20Along%20Spline))
    (LocalVariables|SetAccumulated%20Distance (CallFunction|CalculateNewAccumulatedDistance (LocalVariables|GetAccumulated%20Distance) _offset_distance_between_actors)) ; update Accumulated Distance
  ))

(fn PreviewActorsPlacement
  (bind _scale (Variables|Default|GetScale))
  (LocalVariables|SetAccumulated%20Distance 0.0) ; Initialize Accumulated Distance to 0
  (bind (_number_of_actors_to_place _offset_distance_between_actors) (|CalculateOffsetDistanceAndNumberOfActors(P) _scale (Variables|Default|GetActor%20To%20Spawn)))
  (for _index (range 1 _number_of_actors_to_place)
    (|Preview-SpawnActor _scale (LocalVariables|GetAccumulated%20Distance) (Variables|Default|GetRotate%20Along%20Spline)) ; spawn actor in local space, can serve as preview
    (LocalVariables|SetAccumulated%20Distance (CallFunction|CalculateNewAccumulatedDistance (LocalVariables|GetAccumulated%20Distance) _offset_distance_between_actors)) ; update Accumulated Distance
  ))

(fn CalculateActorSpawnTransformatSplineDistance
  (params (Actor%20Scale :type Vector) (Accumulated%20Distance :type Float%20%28single-precision%29) (Rotate%20Along%20Spline%20Tangent :type Boolean) (Local%20Space%20Transform :type Boolean))
  (if Local%20Space%20Transform
    (LocalVariables|SetCoordinate%20Space "Local"))
  (bind _transform (Math|Transform|MakeTransform (LocalVariables|GetCoordinate%20Space) Accumulated%20Distance Rotate%20Along%20Spline%20Tangent Actor%20Scale)
    (:exit
      (return _transform))))

(fn CalculateNewAccumulatedDistance
  (params (Current%20Accumulated%20Distance :type Float%20%28double-precision%29) (Offset%20Distance%20Between%20Actors :type Float%20%28double-precision%29))
  (return (+ Current%20Accumulated%20Distance Offset%20Distance%20Between%20Actors)))

(fn CalculateActorBoundingBoxDimensionVector
  (params (Actor :type Actor%20Object%20Reference) (Actor%20Scale :type Vector))
  (bind _boxextent (Collision|GetActorBounds Actor false false))
  (return (Math|Vector|VectorGetAbs (* (+ _boxextent _boxextent) Actor%20Scale))))

(fn CalculateOffsetDistanceBetweenActors
  (params (Actor :type Actor%20Object%20Reference) (Actor%20Scale :type Vector))
  (return (+ (|MinimumAllowedDistanceBetweenBoundingBoxesOfTwoActors Actor Actor%20Scale) (Variables|Default|GetSpacing))))

(fn CalculateNumberOfActorstoPlace
  (params (Offset%20Distance%20Between%20Actors :type Float%20%28double-precision%29))
  (return (Math|Float|Ceil (/ (Spline|GetSplineLength (Variables|Default|GetSpline)) Offset%20Distance%20Between%20Actors))))